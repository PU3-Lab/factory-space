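; BP_CharacterPreview is a preview actor that shows an animated character mesh alongside a glowing platform cylinder.
; BeginPlay sets the preview mesh, creates a dynamic material for the platform and starts the looping idle.
; PlayIdle and PlayDance switch looping animations and drive the platform's glow, dim for idle and bright for dance.
; ApplyPreview swaps between woman and man meshes based on IsWoman and plays that character's one-shot hand animation.
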(event `self.ReceiveBeginPlay`
  (`SkeletalMeshComponent.SetSkeletalMeshAsset` (`self.PreviewMesh`) (`self.PreviewSkeletalMesh`))
  (bind _returnvalue (`PrimitiveComponent.CreateDynamicMaterialInstance` (`self.Cylinder`) 0 "/Game/OJJ/Materials/M_Platform.M_Platform" "None"))
  (set `self.PlatformMID` _returnvalue)
  (`self.PlayIdle`))

(fn `ApplyPreview`
  (bind _previewmesh (`self.PreviewMesh`))
  (bind _previewmesh_2 (`self.PreviewMesh`))
  (if (`self.bIsWoman`)
    (`SkeletalMeshComponent.SetSkeletalMeshAsset` _previewmesh_2 "/Game/OJJ/Character/Woman/Woman.Woman")
    (`SkeletalMeshComponent.PlayAnimation` _previewmesh_2 "/Game/OJJ/Character/Woman/Woman_Hand.Woman_Hand" false)
    (else
      (`SkeletalMeshComponent.SetSkeletalMeshAsset` _previewmesh "/Game/OJJ/Character/Man/Man.Man")
      (`SkeletalMeshComponent.PlayAnimation` _previewmesh "/Game/OJJ/Character/Man/Man_Hand.Man_Hand" false))))

(fn `PlayDance`
  (`SkeletalMeshComponent.PlayAnimation` (`self.PreviewMesh`) (`self.DanceAnimation`) true)
  (`MaterialInstanceDynamic.SetScalarParameterValue` (`self.PlatformMID`) "GlowIntensity" 5.0))

(fn `PlayIdle`
  (`SkeletalMeshComponent.PlayAnimation` (`self.PreviewMesh`) (`self.IdleAnimation`) true)
  (`MaterialInstanceDynamic.SetScalarParameterValue` (`self.PlatformMID`) "GlowIntensity" 0.5))

(fn `UserConstructionScript`)